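; AI controller for a simple character that runs the BT_Main06 behavior tree on possession.
; BeginPlay picks a random navigable point near the pawn and stores it in RandomPoint.
; AI Perception updates only print the stimulus tag.
; Nodes that would write the sensed actor to the Blackboard "Player" key or toggle perception are present but unconnected.
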(event OnComponentActivated(AIPerception)
  (params (Component :type Actor%20Component%20Object%20Reference) (bReset :type Boolean)))

(event OnComponentDeactivated(AIPerception)
  (params (Component :type Actor%20Component%20Object%20Reference)))

(event OnTargetPerceptionUpdated(AIPerception)
  (params (Actor :type Actor%20Object%20Reference) (Stimulus :type AI%20Stimulus%20Structure))
  (Development|PrintString (Utilities|String|ToString(Name) (.Tag (Utilities|Struct|BreakAIStimulus Stimulus)))))

(event EventPossess
  (params (PossessedPawn :type Pawn%20Object%20Reference))
  (AI|RunBehaviorTree "/Game/_BP_AI/_Ai06/BT_Main06.BT_Main06"))

(event EventBeginPlay
  (bind _randomlocation (Class|NavigationSystemV1|GetRandomLocationinNavigableRadius (Transformation|GetActorLocation (Pawn|GetControlledPawn)) 3e+02 0 0))
  (Variables|Default|SetRandomPoint _randomlocation))

(fn ConstructionScript)