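; AI controller for a simple character that hands behavior to the BT_Main behavior tree when it possesses a pawn.
; Every tick it emits a noise at the pawn's location through a PawnNoiseEmitter, making the pawn audible to noise sensing.
; Disconnected, unused graphs hold alternative movement approaches: TargetPoint patrol, random navmesh wandering, moving to the player, and line-trace obstacle steering.
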(event EventPossess
  (params (PossessedPawn :type Pawn%20Object%20Reference))
  (AI|RunBehaviorTree "/Game/_BP_AI/_AI04/BT_Main.BT_Main"))

(event EventTick
  (params (DeltaSeconds :type Float%20%28single-precision%29))
  (bind _returnvalue (Pawn|GetControlledPawn))
  (Class|PawnNoiseEmitterComponent|MakeNoise (Variables|Default|GetPawnNoiseEmitter) _returnvalue 1.0 (Transformation|GetActorLocation _returnvalue)))

(fn ConstructionScript)