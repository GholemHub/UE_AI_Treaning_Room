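; AI controller for a simple character that, on BeginPlay, moves toward the first player's pawn with MoveToActor.
; The graph also holds disconnected movement experiments that never run: looping patrol through TargetPoint actors, random reachable-point wandering, and trace-based obstacle steering with AddMovementInput.
; Tick and the construction script are empty.
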(event EventTick
  (params (DeltaSeconds :type Float%20%28single-precision%29)))

(event EventBeginPlay
  (AI|Navigation|MovetoActor self (Game|Player|GetPlayerPawn 0) -1.0 true true true 0))

(fn ConstructionScript)