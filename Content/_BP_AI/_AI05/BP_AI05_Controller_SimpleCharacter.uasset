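; AI controller for a simple character that hands its pawn's behavior to the BT_Main05 behavior tree on possession.
; BeginPlay also stores a random navigable point near the pawn, but only disconnected logic reads it.
; Three unwired movement experiments remain and never run: cycling through TargetPoint actors, wandering between random reachable points, and trace-based steering that rotates movement direction when a forward trace hits.
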(event EventPossess
  (params (PossessedPawn :type Pawn%20Object%20Reference))
  (AI|RunBehaviorTree "/Game/_BP_AI/_AI05/BT_Main05.BT_Main05"))

(event EventTick
  (params (DeltaSeconds :type Float%20%28single-precision%29)))

(event EventBeginPlay
  (bind _randomlocation (Class|NavigationSystemV1|GetRandomLocationinNavigableRadius (Transformation|GetActorLocation (Pawn|GetControlledPawn)) 3e+02 0 0))
  (Variables|Default|SetRandomPoint _randomlocation))

(fn ConstructionScript)