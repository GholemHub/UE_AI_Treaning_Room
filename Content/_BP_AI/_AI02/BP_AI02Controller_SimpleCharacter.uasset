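; AI controller for a simple character that patrols its pawn through the level's TargetPoint actors in a loop.
; Each Tick gathers the TargetPoints and issues AIMoveTo toward the one at PointsIndex.
; On success, a DoN gate advances the index, resetting both itself and the index after the last point.
; Unconnected alternatives remain for random navmesh wandering and trace-based steering that rotates the movement direction on hits.
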(event EventTick
  (params (DeltaSeconds :type Float%20%28single-precision%29))
  (bind _outactors (Actor|GetAllActorsOfClass "/Script/Engine.TargetPoint"))
  (AI|AIMoveTo 0 "0, 0, 0" (Utilities|Array|Get(acopy) _outactors (Variables|Default|GetPointsIndex)) 5.0 false
    (:OnSuccess
      (Utilities|FlowControl|DoN (Utilities|Array|Length _outactors) :!label _label
        (:Exit
          (bind _result (Math|Integer|IncrementInt (Variables|Default|GetPointsIndex))
            (:%20%20
              (Variables|Default|SetPointsIndex _result)
              (if (== (Variables|Default|GetPointsIndex) (Utilities|Array|Length _outactors))
                (Variables|Default|SetPointsIndex 0)
                (goto _label Reset)))))))))

(event EventBeginPlay)

(fn ConstructionScript)