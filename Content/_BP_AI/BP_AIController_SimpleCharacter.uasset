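; AI controller that makes a simple character wander randomly around the navmesh.
; BeginPlay picks a navigable point near the pawn, Tick issues AI MoveTo toward it every frame, and each success picks a new reachable point around the pawn.
; Two disconnected alternatives remain in the graph and never run: a looping TargetPoint patrol and forward-trace steering that randomly rotates the movement direction on a hit.
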(event EventTick
  (params (DeltaSeconds :type Float%20%28single-precision%29))
  (AI|AIMoveTo 0 (Variables|Default|GetRandomPoint) 0 5.0 false
    (:OnSuccess
      (Variables|Default|SetRandomPoint (.RandomLocation (AI|Navigation|GetRandomReachablePointinRadius (Transformation|GetActorLocation (Pawn|GetControlledPawn)) 4e+02 0 0))))))

(event EventBeginPlay
  (bind _randomlocation (Class|NavigationSystemV1|GetRandomLocationinNavigableRadius (Transformation|GetActorLocation (Pawn|GetControlledPawn)) 3e+02 0 0))
  (Variables|Default|SetRandomPoint _randomlocation))

(fn ConstructionScript)